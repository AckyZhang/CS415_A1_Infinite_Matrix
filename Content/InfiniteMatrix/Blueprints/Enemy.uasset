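; Enemy is an actor that wanders randomly, damages the player on contact and can be shot for score.
; On Tick it makes swept moves along Y and Z, re-rolling a random, delta-time-scaled offset whenever a ten-tick counter resets.
; Its sphere overlap either reduces BP_Player health, showing restart on death, or adds the projectile shooter's PassedLastHole to their Score and destroys the projectile.
; Either kind of hit destroys the enemy.
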(event `self.ReceiveTick`
  (params (DeltaSeconds :type "Float (single-precision)"))
  (bind _returnvalue (* DeltaSeconds 500.0))
  (if (== (`self.TickCounter`) 0)
    (set `self.moveY` (* (`KismetMathLibrary.RandomFloatInRange` -1.0 1.0) _returnvalue))
    (set `self.moveZ` (* _returnvalue (`KismetMathLibrary.RandomFloatInRange` -1.0 1.0))))
  (`self.K2_AddActorWorldOffset` (`KismetMathLibrary.MakeVector` 0.0 (`self.moveY`) (`self.moveZ`)) true)
  (bind _result (`/Engine/EditorBlueprintResources/StandardMacros.IncrementInt` (`self.TickCounter`))
    (:`  `
      (if (== _result 10)
        (set `self.TickCounter` 0)))))

(event `self.Sphere.OnComponentBeginOverlap`
  (params (OverlappedComponent :type "PrimitiveComponent Object Reference") (OtherActor :type "Actor Object Reference") (OtherComp :type "PrimitiveComponent Object Reference") (OtherBodyIndex :type Integer) (bFromSweep :type Boolean) (SweepResult :type "HitResult Structure (by ref)"))
  (bind _asbp_player (cast `/Game/InfiniteMatrix/Blueprints/BP_Player` OtherActor)
    (:`then`
      (bind _output_get (set `/Game/InfiniteMatrix/Blueprints/BP_Player.Health` (- (`/Game/InfiniteMatrix/Blueprints/BP_Player.Health` _asbp_player) 20.0) _asbp_player))
      (if (<= _output_get 0.0)
        (set `/Game/InfiniteMatrix/Blueprints/BP_Player.IsDead` true _asbp_player)
        (`/Game/InfiniteMatrix/Blueprints/BP_Player.Display Restart` _asbp_player)))
    (:`CastFailed`
      (bind _asprojectile (cast `/Game/InfiniteMatrix/Blueprints/Projectile` OtherActor))
      (bind _shooter (`/Game/InfiniteMatrix/Blueprints/Projectile.Shooter` _asprojectile))
      (set `/Game/InfiniteMatrix/Blueprints/BP_Player.Score` (+ (`/Game/InfiniteMatrix/Blueprints/BP_Player.Score` _shooter) (`/Game/InfiniteMatrix/Blueprints/BP_Player.PassedLastHole` _shooter)) _shooter)
      (`self.K2_DestroyActor` _asprojectile)))
  (`self.K2_DestroyActor`))

(fn `UserConstructionScript`)